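; Blast door Blueprint with two panels, DoorL and DoorR, that slide apart to open and back together to close.
; OnOpen plays and OnClose reverses a single timeline, whose DoorX track drives both panels' relative X in mirrored directions.
; A normalized DoorPos is scaled by the timeline duration to give a timeline time.
; The construction script calls UpdateDoorPosition, which sets the timeline's time.
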(event Custom|OnOpen
  (bind _doorx (Timeline|Opening_Timeline Play)
    (:Update
      (Transformation|SetRelativeLocation (Variables|Default|GetDoor_L) (Math|Vector|MakeVector (* _doorx -1.0) 0.0 0.0) false false)
      (Transformation|SetRelativeLocation (Variables|Default|GetDoor_R) (Math|Vector|MakeVector _doorx 0.0 0.0) false false))))

(event Custom|OnClose
  (bind _doorx (Timeline|Opening_Timeline Reverse)
    (:Update
      (Transformation|SetRelativeLocation (Variables|Default|GetDoor_L) (Math|Vector|MakeVector (* _doorx -1.0) 0.0 0.0) false false)
      (Transformation|SetRelativeLocation (Variables|Default|GetDoor_R) (Math|Vector|MakeVector _doorx 0.0 0.0) false false))))

(event Custom|UpdateDoorPosition
  (bind _doorx (Timeline|Opening_Timeline SetNewTime)
    (:Update
      (Transformation|SetRelativeLocation (Variables|Default|GetDoor_L) (Math|Vector|MakeVector (* _doorx -1.0) 0.0 0.0) false false)
      (Transformation|SetRelativeLocation (Variables|Default|GetDoor_R) (Math|Vector|MakeVector _doorx 0.0 0.0) false false))))

(event EventBeginPlay)

(event Collision|EventActorBeginOverlap
  (params (OtherActor :type Actor%20Object%20Reference)))

(event EventTick
  (params (DeltaSeconds :type Float%20%28single-precision%29)))

(fn ConstructionScript
  (CallFunction|UpdateDoorPosition))