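; Snakeman enemy monster with a claw attack and a running charge that damages characters it collides with.
; Claw hits damage actors inside the claw hitbox on the server only.
; While running, capsule overlaps with TD characters apply Charge attack damage, or a fallback amount, and fire a radial-push impulse via PushActorsForce.
; A mass-based PushMonster function exists, but its only call in the event graph never runs.
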(event OnComponentBeginOverlap(CapsuleComponent)
  (params (OverlappedComponent :type Primitive%20Component%20Object%20Reference) (OtherActor :type Actor%20Object%20Reference) (OtherComp :type Primitive%20Component%20Object%20Reference) (OtherBodyIndex :type Integer) (bFromSweep :type Boolean) (SweepResult :type Hit%20Result%20Structure%20%28by%20ref%29))
  (bind _returnvalue (Class|TDMonsterCharacter|HasAttackMode (Utilities|Struct|MakeAttackMode "Charge")))
  (if (Variables|Default|GetbIsRunning)
    (bind _astdcharacter (Utilities|Casting|CastToTDCharacter OtherActor))
    (Game|Damage|ApplyDamage _astdcharacter (select (!= _returnvalue -1) (.damage (Utilities|Array|Get(acopy) (Variables|Default|GetAttackModes) _returnvalue)) 1e+01) (Game|GetInstigatorController) self "/Script/Engine.DamageType")
    (Class|RadialForceComponent|FireImpulse (Variables|Default|GetPushActorsForce))))

(event Collision|EventActorBeginOverlap
  (params (OtherActor :type Actor%20Object%20Reference)))

(event EventOnAttackHit
  (params (AttackModeName :type Name :default "None"))
  (Networking|SwitchHasAuthority
    (:Authority
      (Class|TDMonsterCharacter|DamageActorsinVolume (Variables|Default|GetHitClawBox) "Claw"))))

(fn ConstructionScript)