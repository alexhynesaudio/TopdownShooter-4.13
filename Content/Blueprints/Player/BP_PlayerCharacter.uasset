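; BP_PlayerCharacter is the player character, handling camera-relative movement and camera zoom.
; MoveForward and MoveRight axes add movement input along directions built from the SpringArm's relative yaw only, and are ignored while IsDead is true.
; AddCameraHeight zooms by adding a scaled input to the SpringArm's length, clamped to CameraHeightRange.
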(event EventBeginPlay)

(event Collision|EventActorBeginOverlap
  (params (OtherActor :type Actor%20Object%20Reference)))

(event EventTick
  (params (DeltaSeconds :type Float%20%28single-precision%29)))

(event EventAddCameraHeight
  (params (Value :type Float%20%28single-precision%29))
  (bind _cameraheightrange (Variables|Default|GetCameraHeightRange))
  ;[1 1 1] Camera zoom
  (Variables|/Script/Engine.SpringArmComponent|SetTargetArmLength (Variables|Default|GetSpringArm) (Math|Float|Clamp(Float) (+ (* Value 1e+01) (Variables|/Script/Engine.SpringArmComponent|GetTargetArmLength (Variables|Default|GetSpringArm))) (.x _cameraheightrange) (.y _cameraheightrange))))

(event Input|AxisEvents|InputAxisMoveForward
  (params (AxisValue :type Float%20%28single-precision%29))
  ;[1 1 1] Move forward
  (if (not (Class|TDCharacter|IsDead))
    (Pawn|Input|AddMovementInput (Math|Vector|GetForwardVector (Math|Rotator|MakeRotator 0.0 0.0 (.yaw (Variables|/Script/Engine.SceneComponent|GetRelativeRotation (Variables|Default|GetSpringArm))))) AxisValue false)))

(event Input|AxisEvents|InputAxisMoveRight
  (params (AxisValue :type Float%20%28single-precision%29))
  ;[1 1 1] Move right
  (if (not (Class|TDCharacter|IsDead))
    (Pawn|Input|AddMovementInput (Math|Vector|GetRightVector (Math|Rotator|MakeRotator 0.0 0.0 (.yaw (Variables|/Script/Engine.SceneComponent|GetRelativeRotation (Variables|Default|GetSpringArm))))) AxisValue false)))

(fn ConstructionScript)