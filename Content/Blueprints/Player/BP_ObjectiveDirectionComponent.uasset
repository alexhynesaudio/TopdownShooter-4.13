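; Player component that draws a debug arrow pointing the local player toward the current objective.
; Each tick it skips dead characters, reads CurrentObjective from TDGameState and only draws for the locally controlled player.
; The direction is flattened to the horizontal plane, so the short translucent blue arrow floats just ahead of the character at the actor's height.
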(event EventBeginPlay)

(event EventTick
  (params (DeltaSeconds :type Float%20%28single-precision%29))
  (bind _returnvalue (Components|GetOwner))
  (bind _returnvalue_2 (Transformation|GetActorLocation _returnvalue))
  (bind _returnvalue_3 (Transformation|GetActorLocation _returnvalue))
  (bind _astdplayer_character (Utilities|Casting|CastToTDPlayerCharacter (Components|GetOwner)))
  (if (not (Class|TDCharacter|IsDead _astdplayer_character))
    (bind _astdgame_state (Utilities|Casting|CastToTDGameState (Game|GetGameState)))
    (Utilities|IsValid (Variables|/Script/TopDownShooter.TDGameState|GetCurrentObjective _astdgame_state)
      (:Is%20Valid
        (if (Pawn|IsLocalController (Pawn|GetController (Variables|/Script/Engine.Actor|GetInstigator _returnvalue)))
          (Rendering|Debug|DrawDebugArrow (+ _returnvalue_2 (* (Class|KismetMathLibrary|GetDirectionVector (Math|Vector|MakeVector (.x _returnvalue_3) (.y _returnvalue_3) 0.0) (Math|Vector|MakeVector (.x (Transformation|GetActorLocation (Variables|/Script/TopDownShooter.TDGameState|GetCurrentObjective _astdgame_state))) (.y (Transformation|GetActorLocation (Variables|/Script/TopDownShooter.TDGameState|GetCurrentObjective _astdgame_state))) 0.0)) 8e+01)) (+ _returnvalue_2 (* (Class|KismetMathLibrary|GetDirectionVector (Math|Vector|MakeVector (.x _returnvalue_3) (.y _returnvalue_3) 0.0) (Math|Vector|MakeVector (.x (Transformation|GetActorLocation (Variables|/Script/TopDownShooter.TDGameState|GetCurrentObjective _astdgame_state))) (.y (Transformation|GetActorLocation (Variables|/Script/TopDownShooter.TDGameState|GetCurrentObjective _astdgame_state))) 0.0)) 1.2e+02)) 1e+02 "(R=0.362755,G=0.628008,B=0.980000,A=0.400000)" 0.0 1e+01))))))