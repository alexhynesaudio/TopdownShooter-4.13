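; Player helper that draws direction arrows around its owner, pointing toward every other TDPlayerCharacter in the level.
; On Tick, only when the owner's instigator controller is local, it gathers all player characters and skips the owner.
; Directions are computed on the XY plane, and each becomes a short translucent green arrow offset from the owner's location.
; The arrows are rendered with DrawDebugArrow rather than meshes or UI.
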(event EventBeginPlay)

(event EventTick
  (params (DeltaSeconds :type Float%20%28single-precision%29))
  (bind _returnvalue (Components|GetOwner))
  (bind _returnvalue_2 (Transformation|GetActorLocation _returnvalue))
  (bind _returnvalue_3 (Transformation|GetActorLocation _returnvalue))
  (if (Pawn|IsLocalController (Pawn|GetController (Variables|/Script/Engine.Actor|GetInstigator _returnvalue)))
    (bind _outactors (Actor|GetAllActorsOfClass "/Script/TopDownShooter.TDPlayerCharacter"))
    (for _array_element _outactors
      (if (not (== _array_element _returnvalue))
        (Rendering|Debug|DrawDebugArrow (+ _returnvalue_2 (* (Class|KismetMathLibrary|GetDirectionVector (Math|Vector|MakeVector (.x _returnvalue_3) (.y _returnvalue_3) 0.0) (Math|Vector|MakeVector (.x (Transformation|GetActorLocation _array_element)) (.y (Transformation|GetActorLocation _array_element)) 0.0)) 6e+01)) (+ _returnvalue_2 (* (Class|KismetMathLibrary|GetDirectionVector (Math|Vector|MakeVector (.x _returnvalue_3) (.y _returnvalue_3) 0.0) (Math|Vector|MakeVector (.x (Transformation|GetActorLocation _array_element)) (.y (Transformation|GetActorLocation _array_element)) 0.0)) 8e+01)) 4e+01 "(R=0.127400,G=0.980000,B=0.390335,A=0.400000)" 0.0 5.0)))))